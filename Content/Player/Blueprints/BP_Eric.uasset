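; Player Blueprint for Eric that handles pausing, item tutorial prompts and disabling the HUD.
; P, Escape and gamepad Special Right each lazily create a cached PauseMenu, switch input to UI, pause the game and focus Resume.
; Remote, screwdriver and knife tutorial events use boolean flags to play their BP_TutorialWidget animation only once.
; DiableHUD casts the player's HUD to EricHUD and sets its DisableHud flag.
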(event `Key|P`
  (params (Key :type "Key Structure" :default "AnyKey"))
  (bind _pausemenureference (`self.PauseMenuReference`))
  (:`Pressed`
    (`/Engine/EditorBlueprintResources/StandardMacros.IsValid` (`self.PauseMenuReference`)
      (:`Is Valid`
        _)
      (:`Is Not Valid`
        (bind _returnvalue (`|CreateWidget` "/Game/UI/PauseMenu.PauseMenu_C"))
        (set `self.PauseMenuReference` _returnvalue)))
    (`WidgetBlueprintLibrary.SetInputMode_UIOnlyEx` (`GameplayStatics.GetPlayerController` null) _pausemenureference)
    (`UserWidget.AddToViewport` _pausemenureference 0)
    (`GameplayStatics.SetGamePaused` null true)
    (`Widget.SetKeyboardFocus` (`/Game/UI/PauseMenu.ResumeButton` _returnvalue))
    (set `PlayerController.bShowMouseCursor` true (`GameplayStatics.GetPlayerController` null))))

(event `Key|Escape`
  (params (Key :type "Key Structure" :default "AnyKey"))
  (bind _pausemenureference (`self.PauseMenuReference`))
  (:`Pressed`
    (`/Engine/EditorBlueprintResources/StandardMacros.IsValid` (`self.PauseMenuReference`)
      (:`Is Valid`
        _)
      (:`Is Not Valid`
        (bind _returnvalue (`|CreateWidget` "/Game/UI/PauseMenu.PauseMenu_C"))
        (set `self.PauseMenuReference` _returnvalue)))
    (`WidgetBlueprintLibrary.SetInputMode_UIOnlyEx` (`GameplayStatics.GetPlayerController` null) _pausemenureference)
    (`UserWidget.AddToViewport` _pausemenureference 0)
    (`GameplayStatics.SetGamePaused` null true)
    (`Widget.SetKeyboardFocus` (`/Game/UI/PauseMenu.ResumeButton` _returnvalue))
    (set `PlayerController.bShowMouseCursor` true (`GameplayStatics.GetPlayerController` null))))

(event `Key|Gamepad_Special_Right`
  (params (Key :type "Key Structure" :default "AnyKey"))
  (bind _pausemenureference (`self.PauseMenuReference`))
  (:`Pressed`
    (`/Engine/EditorBlueprintResources/StandardMacros.IsValid` (`self.PauseMenuReference`)
      (:`Is Valid`
        _)
      (:`Is Not Valid`
        (bind _returnvalue (`|CreateWidget` "/Game/UI/PauseMenu.PauseMenu_C"))
        (set `self.PauseMenuReference` _returnvalue)))
    (`WidgetBlueprintLibrary.SetInputMode_UIOnlyEx` null _pausemenureference)
    (`UserWidget.AddToViewport` _pausemenureference 0)
    (`GameplayStatics.SetGamePaused` null true)
    (`Widget.SetKeyboardFocus` (`/Game/UI/PauseMenu.ResumeButton` _returnvalue))
    (set `PlayerController.bShowMouseCursor` true (`GameplayStatics.GetPlayerController` null))))

(event `self.ReceiveActorBeginOverlap`
  (params (OtherActor :type "Actor Object Reference")))

(event `self.ShowRemoteTutorial`
  (if (`self.bRemotetut`)
    (bind _returnvalue (`|CreateWidget` "/Game/UI/BP_TutorialWidget.BP_TutorialWidget_C"))
    (`UserWidget.AddToViewport` _returnvalue 0)
    (`UserWidget.PlayAnimation` _returnvalue (`/Game/UI/BP_TutorialWidget.ShowRemoteTutorial` _returnvalue) 0.0 1 "Forward")
    (set `self.bRemotetut` false)))

(event `self.ShowScrewDriverTutorial`
  (if (`self.bScrewdrivertut`)
    (bind _returnvalue (`|CreateWidget` "/Game/UI/BP_TutorialWidget.BP_TutorialWidget_C"))
    (`UserWidget.AddToViewport` _returnvalue 0)
    (`UserWidget.PlayAnimation` _returnvalue (`/Game/UI/BP_TutorialWidget.ShowScrewdriverTutorial` _returnvalue) 0.0 1 "Forward")
    (set `self.bScrewdrivertut` false)))

(event `self.ShowKnifeTutorial`
  (if (`self.bKnifetut`)
    (bind _returnvalue (`|CreateWidget` "/Game/UI/BP_TutorialWidget.BP_TutorialWidget_C"))
    (`UserWidget.AddToViewport` _returnvalue 0)
    (`UserWidget.PlayAnimation` _returnvalue (`/Game/UI/BP_TutorialWidget.ShowKnifeTutorial` _returnvalue) 0.0 1 "Forward")
    (set `self.bKnifetut` false)))

(fn `DiableHUD`
  (bind _aseric_hud (cast `EricHUD` (`PlayerController.GetHUD` (`GameplayStatics.GetPlayerController` null))))
  (set `EricHUD.bDisableHud` true _aseric_hud))

(fn `UserConstructionScript`)
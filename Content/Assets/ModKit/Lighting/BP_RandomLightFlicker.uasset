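; Point light Blueprint that flickers at random intervals, toggling the light on and off with audio feedback.
; Tick drives a Delay of a random length under one second, then flips the point light component's visibility.
; Switching on plays the LightOn sound, while switching off calls Play after setting an empty sound.
; BeginPlay and the construction script are empty, and an unused copy of the flicker logic remains in the graph.
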(event `self.ReceiveTick`
  (params (DeltaSeconds :type "Float (single-precision)"))
  (bind _pointlightcomponent (`self.PointLightComponent`))
  (bind _output_get (set `self.Duration` (`KismetMathLibrary.RandomFloat`)))
  (`KismetSystemLibrary.Delay` _output_get)
  (if (`SceneComponent.IsVisible` (`self.PointLightComponent`))
    (`SceneComponent.SetVisibility` _pointlightcomponent false false)
    (`AudioComponent.SetSound` (`self.AudioComp`) null)
    (`AudioComponent.Play` (`self.AudioComp`) 0.0)
    (else
      (`SceneComponent.SetVisibility` _pointlightcomponent true false)
      (`AudioComponent.SetSound` (`self.AudioComp`) "/Game/Sounds/Environment/LightOn.LightOn")
      (`AudioComponent.Play` (`self.AudioComp`) 0.0))))

(event `ReceiveBeginPlay_Copy`)

(event `self.ReceiveBeginPlay`)

(fn `UserConstructionScript`)